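; Player-controlled mech Blueprint that puts the main screen UI on the viewport and carries debug hotkeys for its current weapon.
; BeginPlay creates and adds the MainScreen widget.
; Key 1 sets the mech as owner of MCurrentWeapon, and key 3 prints that weapon's ammo and clip values in separate colors.
; Tick and TimerHandleTest are empty, and leftover test nodes for authority, tracing and ammo use are unconnected.
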(event `self.ReceiveBeginPlay`
  (bind _returnvalue (`|CreateWidget` "/Game/UI/PlayerHud/MainScreen.MainScreen_C"))
  (`UserWidget.AddToViewport` _returnvalue 0))

(event `self.ReceiveTick`
  (params (DeltaSeconds :type "Float (single-precision)")))

(event `Key|One`
  (params (Key :type "Key Structure" :default "AnyKey"))
  (:`Pressed`
    (`self.SetOwner` (`self.m_CurrentWeapon`) self)))

(event `Key|Three`
  (params (Key :type "Key Structure" :default "AnyKey"))
  (bind _m_currentweapon (`self.m_CurrentWeapon`))
  (:`Pressed`
    (`KismetSystemLibrary.PrintString` (`KismetStringLibrary.Conv_IntToString` (`Weapon_Base.m_CurrentAmmo` _m_currentweapon)) true true (struct :`R` 1.0 :`A` 1.0))
    (`KismetSystemLibrary.PrintString` (`KismetStringLibrary.Conv_IntToString` (`Weapon_Base.m_AmmosInClip` _m_currentweapon)) true true (struct :`G` 1.0 :`A` 1.0))
    (`KismetSystemLibrary.PrintString` (`KismetStringLibrary.Conv_IntToString` (`Weapon_Base.m_CurrentClip` _m_currentweapon)) true true (struct :`B` 1.0 :`A` 1.0))))

(fn `TimerHandleTest`)

(fn `UserConstructionScript`)